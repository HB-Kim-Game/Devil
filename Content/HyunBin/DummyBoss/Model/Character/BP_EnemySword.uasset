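; BP_EnemySword is an enemy's sword actor that deals melee damage and carries an attached lightning Niagara effect.
; SetSwordTrace toggles a looping sphere trace along the blade, which stops after its first damaging hit.
; ChargingSwordTrace is a one-shot, wider, stronger trace using the kick damage type, while Start/EndCharging toggle an overlay mesh.
; Hits slow global time and start a spawned BP_CustomTimer for hit-stop.
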(event `self.ReceiveBeginPlay`
  (bind _returnvalue (`|SpawnActorFromClass` "/Game/HyunBin/DummyBoss/Blueprints/BP_CustomTimer.BP_CustomTimer_C" (`self.GetTransform`) "AlwaysSpawn" "MultiplyWithRoot" null null))
  (set `self.Timer` _returnvalue)
  (bind _returnvalue_2 (`NiagaraFunctionLibrary.SpawnSystemAttached` "/Game/HyunBin/VFX/ModelVFX/NS_LightningSword.NS_LightningSword" (`self.SwordBottom`) "None" (`SceneComponent.K2_GetComponentLocation` (`self.SwordBottom`)) (`SceneComponent.K2_GetComponentRotation` (`self.SwordBottom`)) "KeepWorldPosition"))
  (set `self.Effect` _returnvalue_2))

(event `SetSwordTrace`
  (params (State :type Boolean))
  (bind _tracehandle (`self.TraceHandle`))
  (if State
    (bind _returnvalue (`KismetSystemLibrary.K2_SetTimerDelegate` (delegate `SwordTrace`) 0.01 true))
    (set `self.TraceHandle` _returnvalue)
    (elif (`KismetSystemLibrary.K2_IsValidTimerHandle` _tracehandle)
      (`KismetSystemLibrary.K2_ClearAndInvalidateTimerHandle` _tracehandle))))

(event `SwordTrace`
  (bind (_outhit _returnvalue) (`KismetSystemLibrary.SphereTraceSingle` (`SceneComponent.K2_GetComponentLocation` (`self.SwordTop`)) (`SceneComponent.K2_GetComponentLocation` (`self.SwordBottom`)) 30.0 "TraceTypeQuery1"))
  (if _returnvalue
    (bind (_bblockinghit _binitialoverlap _time _distance _location _impactpoint _normal _impactnormal _physmat _hitactor _hitcomponent _hitbonename _bonename _hititem _elementindex _faceindex _tracestart) (`GameplayStatics.BreakHitResult` _outhit))
    (if (`|EnumEquality` (`PrimitiveComponent.GetCollisionObjectType` _hitcomponent) "ECC_GameTraceChannel2")
      (`GameplayStatics.ApplyPointDamage` _hitactor 10.0 _tracestart _outhit null (`self.Enemy`) "/Game/MinSoo/Blueprints/BP_DT_EnemySlash.BP_DT_EnemySlash_C")
      (`KismetSystemLibrary.PrintString` "Damage")
      (`GameplayStatics.SetGlobalTimeDilation` 0.4)
      (`/Game/HyunBin/DummyBoss/Blueprints/BP_CustomTimer.TimerStart` (`self.Timer`) 0.025)
      (`KismetSystemLibrary.K2_ClearAndInvalidateTimerHandle` (`self.TraceHandle`)))))

(event `StartCharging`
  (`SceneComponent.SetVisibility` (`self.OverlayMesh`) true false))

(event `EndCharging`
  (`SceneComponent.SetVisibility` (`self.OverlayMesh`) false false))

(event `ChargingSwordTrace`
  (bind (_returnvalue_x _returnvalue_y _returnvalue_z) (`KismetMathLibrary.BreakVector` (`SceneComponent.K2_GetComponentLocation` (`self.SwordTop`))))
  (bind (_outhit _returnvalue) (`KismetSystemLibrary.SphereTraceSingle` (`SceneComponent.K2_GetComponentLocation` (`self.SwordBottom`)) (`KismetMathLibrary.MakeVector` _returnvalue_x _returnvalue_y (+ _returnvalue_z 50.0)) 75.0 "TraceTypeQuery1"))
  (if _returnvalue
    (bind (_bblockinghit _binitialoverlap _time _distance _location _impactpoint _normal _impactnormal _physmat _hitactor _hitcomponent _hitbonename _bonename _hititem _elementindex _faceindex _tracestart) (`GameplayStatics.BreakHitResult` _outhit))
    (if (`|EnumEquality` (`PrimitiveComponent.GetCollisionObjectType` _hitcomponent) "ECC_GameTraceChannel2")
      (`GameplayStatics.ApplyPointDamage` _hitactor 50.0 _tracestart _outhit null (`self.Enemy`) "/Game/MinSoo/Blueprints/BP_DT_EnemyKick.BP_DT_EnemyKick_C")
      (`KismetSystemLibrary.PrintString` "Damage")
      (`GameplayStatics.SetGlobalTimeDilation` 0.4)
      (`/Game/HyunBin/DummyBoss/Blueprints/BP_CustomTimer.TimerStart` (`self.Timer`) 0.033))))

(fn `UserConstructionScript`)