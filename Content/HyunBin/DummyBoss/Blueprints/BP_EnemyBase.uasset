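; Base enemy character for a sword-wielding boss, driven by BP_AIC_EnemyBase, which receives damage, frozen and death states.
; Montage chains drive a slash-slash-kick combo and directional hit reactions, alongside a projectile aimed at the blackboard target.
; The kick sphere-traces for point damage, adding slow motion and camera shake on hit.
; It also provides timer-spawned afterimages, a kill camera, timeline-eased time dilation, and range, patrol and speed queries.
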(event `self.ReceiveTick`
  (params (DeltaSeconds :type "Float (single-precision)")))

(event `self.ReceiveBeginPlay`
  (bind _asbp_aic_enemy_base (cast `/Game/HyunBin/DummyBoss/Blueprints/AI/BP_AIC_EnemyBase` (`self.GetController`)))
  (set `self.BossController` _asbp_aic_enemy_base)
  (`self.EquipSword`)
  (bind _returnvalue (`|SpawnActorFromClass` "/Game/HyunBin/DummyBoss/Blueprints/BP_CustomTimer.BP_CustomTimer_C" (`self.GetTransform`) "AlwaysSpawn" "MultiplyWithRoot" null null))
  (set `self.TestTimer` _returnvalue)
  (`/Game/HyunBin/DummyBoss/Blueprints/AI/BP_AIC_EnemyBase.SetHitState` (`self.BossController`))
  (set `self.CurrentHP` (`self.MaxHP`)))

(event `SetSpawnAfterEffect`
  (params (State :type Boolean))
  (bind _spawntimer (`self.SpawnTimer`))
  (if State
    (bind _returnvalue (`KismetSystemLibrary.K2_SetTimerDelegate` (delegate `SpawnAfterImage`) 0.1 true))
    (set `self.SpawnTimer` _returnvalue)
    (elif (`KismetSystemLibrary.K2_IsValidTimerHandle` _spawntimer)
      (`KismetSystemLibrary.K2_ClearAndInvalidateTimerHandle` _spawntimer))))

(event `SpawnAfterImage`
  (bind _returnvalue (`|SpawnActorFromClass` "/Game/HyunBin/DummyBoss/Blueprints/BP_AfterImage.BP_AfterImage_C" (`SceneComponent.K2_GetComponentToWorld` (`self.Mesh`)) "AlwaysSpawn" "MultiplyWithRoot" null null))
  (`/Game/HyunBin/DummyBoss/Blueprints/BP_AfterImage.SetCharacter` _returnvalue self)
  (`/Game/HyunBin/DummyBoss/Blueprints/BP_AfterImage.Activate` _returnvalue))

(event `SetSwordTrace`
  (params (State :type Boolean))
  (`/Game/HyunBin/DummyBoss/Model/Character/BP_EnemySword.SetSwordTrace` (`self.Sword`) State))

(event `KickTrace`
  (bind _mesh (`self.Mesh`))
  (bind _returnvalue (`SceneComponent.GetSocketLocation` _mesh "RightToeBase"))
  (bind (_returnvalue_roll _returnvalue_pitch _returnvalue_yaw) (`KismetMathLibrary.BreakRotator` (`KismetMathLibrary.MakeRotFromXZ` (`self.GetActorForwardVector`) (`self.GetActorUpVector`))))
  (bind _returnvalue_2 (`NiagaraFunctionLibrary.SpawnSystemAtLocation` "/Game/HyunBin/VFX/AttackVFX/NS_Shockwave.NS_Shockwave" _returnvalue (`KismetMathLibrary.MakeRotator` _returnvalue_roll -90.0 _returnvalue_yaw)))
  (`NiagaraComponent.SetCustomTimeDilation` _returnvalue_2 2.2)
  (bind (_outhit _returnvalue_3) (`KismetSystemLibrary.SphereTraceSingle` (`SceneComponent.GetSocketLocation` _mesh "RightFoot") _returnvalue 60.0 "TraceTypeQuery1"))
  (if _returnvalue_3
    (bind (_bblockinghit _binitialoverlap _time _distance _location _impactpoint _normal _impactnormal _physmat _hitactor _hitcomponent _hitbonename _bonename _hititem _elementindex _faceindex _tracestart) (`GameplayStatics.BreakHitResult` _outhit))
    (if (`|EnumEquality` (`PrimitiveComponent.GetCollisionObjectType` _hitcomponent) "ECC_GameTraceChannel2")
      (`GameplayStatics.ApplyPointDamage` _hitactor 20.0 _tracestart _outhit null self "/Game/MinSoo/Blueprints/BP_DT_EnemyKick.BP_DT_EnemyKick_C")
      (`KismetSystemLibrary.PrintString` "Damage")
      (`GameplayStatics.SetGlobalTimeDilation` 0.4)
      (`/Game/HyunBin/DummyBoss/Blueprints/BP_CustomTimer.TimerStart` (`self.TestTimer`) 0.033)
      (`GameplayStatics.PlayWorldCameraShake` "/Game/HyunBin/DummyBoss/Blueprints/CameraShake/BP_EnemyStrongShake.BP_EnemyStrongShake_C" (`self.K2_GetActorLocation`) 0.0 2000.0))))

(event `BallAttack`
  (bind _returnvalue (`|SpawnActorFromClass` "/Game/HyunBin/DummyBoss/Blueprints/Attack/BP_EnemyProjectile.BP_EnemyProjectile_C" (`SceneComponent.GetSocketTransform` (`self.Mesh`) "LeftHand" "RTS_World") "AlwaysSpawn" "MultiplyWithRoot" null null))
  (`/Engine/EditorBlueprintResources/StandardMacros.IsValid` _returnvalue
    (:`Is Valid`
      (set `/Game/HyunBin/DummyBoss/Blueprints/Attack/BP_EnemyProjectile.Enemy` self _returnvalue)
      (`self.K2_SetActorLocation` _returnvalue (+ (* (`self.GetActorForwardVector` _returnvalue) 20.0) (`self.K2_GetActorLocation` _returnvalue)) true false)
      (bind _asactor (cast `Actor` (`BlackboardComponent.GetValueAsObject` (`AIController.Blackboard` (`self.BossController`)) (`self.AttackTargetName`))))
      (`/Game/HyunBin/DummyBoss/Blueprints/Attack/BP_EnemyProjectile.SetAttackTarget` _returnvalue _asactor))))

(event `Attack`
  (bind _mesh (`self.Mesh`))
  (`|PlayMontage` _mesh "/Game/HyunBin/DummyBoss/Animation/sword_and_shield_slash_Montage.sword_and_shield_slash_Montage" 1.0 0.0 "None" false
    (:`OnCompleted`
      (`|PlayMontage` _mesh "/Game/HyunBin/DummyBoss/Animation/sword_and_shield_slash_3_Montage.sword_and_shield_slash_3_Montage" 1.0 0.0 "None" false
        (:`OnCompleted`
          (`|PlayMontage` _mesh "/Game/HyunBin/DummyBoss/Animation/sword_and_shield_kick_Montage.sword_and_shield_kick_Montage" 1.0 0.0 "None" false
            (:`OnCompleted`
              _)
            (:`OnInterrupted`
              _))
          (`self.OnAttackEnd`))))))

(event `PlayImpact`
  (bind _mesh (`self.Mesh`))
  (`MovementComponent.StopMovementImmediately` (`self.CharacterMovement`))
  (if (> (`KismetMathLibrary.Dot_VectorVector` (`KismetMathLibrary.Normal` (- (`self.HitLocation`) (`self.K2_GetActorLocation`))) (`self.GetActorForwardVector`)) 0.0)
    (`|PlayMontage` _mesh "/Game/HyunBin/DummyBoss/Animation/sword_and_shield_impact_3_Montage.sword_and_shield_impact_3_Montage" 1.0 0.1
      (:`OnCompleted`
        _)
      (:`OnInterrupted`
        _))
    (else
      (`|PlayMontage` _mesh "/Game/HyunBin/DummyBoss/Animation/sword_and_shield_impact_2_Montage.sword_and_shield_impact_2_Montage"
        (:`OnCompleted`
          _)
        (:`OnInterrupted`
          _))))
  (`self.OnPlayImpactEnd`))

(event `FinisherTimer`
  (params (Slow :type Boolean))
  (if Slow
    (bind (_direction _timespeed) (`Timeline|SmoothTime` :!label _label)
      (:`Update`
        (`GameplayStatics.SetGlobalTimeDilation` _timespeed)))
    (else
      (goto _label :!via `Reverse`))))

(event `self.ReceivePointDamage`
  (params (Damage :type "Float (single-precision)") (DamageType :type "DamageType Object Reference") (HitLocation :type "Vector Structure") (HitNormal :type "Vector Structure") (HitComponent :type "PrimitiveComponent Object Reference") (BoneName :type Name) (ShotFromDirection :type "Vector Structure") (InstigatedBy :type "Controller Object Reference") (DamageCauser :type "Actor Object Reference") (HitInfo :type "HitResult Structure (by ref)"))
  (bind _bosscontroller (`self.BossController`))
  (`self.SpawnHitEffect` HitInfo_ImpactPoint)
  (bind _output_get (set `self.CurrentHP` (- (`self.CurrentHP`) Damage)))
  (if (<= _output_get 0.1)
    (`/Game/HyunBin/DummyBoss/Blueprints/AI/BP_AIC_EnemyBase.SetStateAsDead` (`self.BossController`))
    (else
      (`/Game/HyunBin/DummyBoss/Blueprints/AI/BP_AIC_EnemyBase.AddDamage` _bosscontroller Damage)
      (`/Game/HyunBin/DummyBoss/Blueprints/AI/BP_AIC_EnemyBase.SetStateAsFrozen` _bosscontroller))))

(fn `EquipSword`
  (bind _returnvalue (`|SpawnActorFromClass` "/Game/HyunBin/DummyBoss/Model/Character/BP_EnemySword.BP_EnemySword_C" (`self.GetTransform`) "AlwaysSpawn" "MultiplyWithRoot" null null))
  (bind _output_get (set `self.Sword` _returnvalue))
  (`self.K2_AttachToComponent` _output_get (`self.Mesh`) "RightHandSocket" "KeepWorld" "KeepRelative" "KeepRelative" true)
  (set `/Game/HyunBin/DummyBoss/Model/Character/BP_EnemySword.Enemy` self _returnvalue))

(fn `GetIdealRange`
  (returns (AttackRadius :type "Float (double-precision)") (DefendRadius :type "Float (double-precision)"))
  (return 300.0 2000.0))

(fn `GetPatrolRoute`
  (returns (Route :type "/Game/HyunBin/DummyBoss/Blueprints/AI/BP_PatrolRoute Object Reference"))
  (return (`self.PatrolRoute`)))

(fn `PlayerDead`
  (`BrainComponent.StopLogic` (`AIController.BrainComponent` (`AIBlueprintHelperLibrary.GetAIController` self)) ""))

(fn `SetKillCamera`
  (params (Begin :type Boolean))
  (locals (Player :type "/Game/MinSoo/Blueprints/BP_MyCharacter Object Reference"))
  (bind _returnvalue (`GameplayStatics.GetPlayerPawn` 0))
  (bind _returnvalue_2 (`GameplayStatics.GetPlayerController` 0))
  (bind _camera (`self.Camera`))
  (bind _returnvalue_3 (`self.K2_GetActorLocation` _returnvalue))
  (bind _returnvalue_4 (+ (- _returnvalue_3 (* (`self.GetActorRightVector` _returnvalue) 320.0)) (-200.0 0.0 110.0)))
  (if Begin
    (`SceneComponent.K2_SetWorldLocationAndRotation` _camera _returnvalue_4 (`KismetMathLibrary.MakeRotator` (- (.roll (`KismetMathLibrary.FindLookAtRotation` _returnvalue_4 _returnvalue_3)) 10.0) (.pitch (`KismetMathLibrary.FindLookAtRotation` _returnvalue_4 _returnvalue_3)) (.yaw (`KismetMathLibrary.FindLookAtRotation` _returnvalue_4 _returnvalue_3))) false false)
    (`PlayerController.SetViewTargetWithBlend` _returnvalue_2 (`ActorComponent.GetOwner` _camera) 0.5 "VTBlend_Linear" 0.0 false)
    (else
      (`PlayerController.SetViewTargetWithBlend` _returnvalue_2 _returnvalue 0.75 "VTBlend_Linear" 0.0 false))))

(fn `SetMovementSpeed`
  (params (Speed :type "/Game/HyunBin/DummyBoss/Blueprints/AI/Enum/E_MovementSpeed Enum" :default "NewEnumerator0"))
  (returns (SpeedValue :type "Float (double-precision)"))
  (bind _output_get (set `CharacterMovementComponent.MaxWalkSpeed` (select `/Game/HyunBin/DummyBoss/Blueprints/AI/Enum/E_MovementSpeed` Speed :`NewEnumerator1` 300.0 :`NewEnumerator2` 2000.0 :`NewEnumerator3` 500.0) (`self.CharacterMovement`)))
  (return _output_get))

(fn `SpawnHitEffect`
  (params (Location :type "Vector Structure"))
  (`GameplayStatics.SpawnEmitterAtLocation` "/Game/HyunBin/VFX/Realistic_Starter_VFX_Pack_Vol2/Particles/Destruction/P_Destruction_Electric.P_Destruction_Electric" Location (struct) (0.5 0.5 0.5))
  (set `self.HitLocation` Location))

(fn `SpawnSwordTracePoint`
  (bind _mesh (`self.Mesh`))
  (bind _returnvalue (`AddComponent|NODE_AddArrowComponent-0`))
  (bind _output_get (set `self.SwordTop` _returnvalue))
  (`SceneComponent.K2_AttachToComponent` _output_get _mesh "Sword_Top" "KeepRelative" "KeepRelative" "KeepRelative" true)
  (bind _returnvalue_2 (`AddComponent|NODE_AddArrowComponent-1`))
  (bind _output_get_2 (set `self.SwordBottom` _returnvalue_2))
  (`SceneComponent.K2_AttachToComponent` _output_get_2 _mesh "Sword_Bottom" "KeepRelative" "KeepRelative" "KeepRelative" true))

(fn `Unpause`
  (`GameplayStatics.SetGamePaused` false))

(fn `UserConstructionScript`)