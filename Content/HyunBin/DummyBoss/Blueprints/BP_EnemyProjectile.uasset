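; BP_EnemyProjectile is an enemy projectile that flies in a straight line and bursts on overlap.
; SetAttackTarget turns it once toward the target's current location, and Tick sweeps it forward at Speed with no homing.
; It attaches a trail effect on BeginPlay, and any actor overlap spawns an impact effect and destroys it, with no damage applied here.
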(event `self.ReceiveBeginPlay`
  (bind _returnvalue (`NiagaraFunctionLibrary.SpawnSystemAttached` "/Game/HyunBin/VFX/SwordTrailVFX/VFX/NS_Trail_08.NS_Trail_08" (`self.Sphere`) "None" (0.0 0.0 0.0) (struct) "KeepRelativeOffset" true))
  (`SceneComponent.K2_SetRelativeLocation` _returnvalue (0.0 0.0 -70.0) true false))

(event `self.ReceiveActorBeginOverlap`
  (params (OtherActor :type "Actor Object Reference"))
  (bind _returnvalue (`NiagaraFunctionLibrary.SpawnSystemAtLocation` "/Game/HyunBin/VFX/Basic_VFX/Custom/CustomEffect_2.CustomEffect_2" (`self.K2_GetActorLocation`) (struct) (0.5 0.5 0.5)))
  (`NiagaraComponent.SetCustomTimeDilation` _returnvalue 1.5)
  (`self.K2_DestroyActor`))

(event `self.ReceiveTick`
  (params (DeltaSeconds :type "Float (single-precision)"))
  (`self.K2_SetActorLocation` (+ (`self.K2_GetActorLocation`) (* (`self.Speed`) DeltaSeconds (`self.GetActorForwardVector`))) true))

(fn `SetAttackTarget`
  (params (Target :type "Actor Object Reference"))
  (bind _output_get (set `self.AttackTarget` Target))
  (bind _output_get_2 (set `self.TargetLocation` (`self.K2_GetActorLocation` _output_get)))
  (`self.K2_SetActorRotation` (`KismetMathLibrary.MakeRotFromXZ` (`KismetMathLibrary.Normal` (- _output_get_2 (`self.K2_GetActorLocation`))) (`self.GetActorUpVector`))))

(fn `UserConstructionScript`)