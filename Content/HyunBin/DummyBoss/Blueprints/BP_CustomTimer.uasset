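; BP_CustomTimer is a timer Blueprint in the DummyBoss folder that restores global time dilation to normal after a given duration.
; TimerStart stores the duration and starts a looping 0.02-second timer on PlayingTimer, keeping its handle.
; PlayingTimer adds that fixed step to a counter and, on reaching the duration, resets the counter, clears the timer and sets time dilation to 1.
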(event `self.ReceiveBeginPlay`)

(event `self.ReceiveTick`
  (params (DeltaSeconds :type "Float (single-precision)")))

(fn `PlayingTimer`
  (bind _output_get (set `self.CurrentTime` (+ (`self.CurrentTime`) 0.02)))
  (if (>= _output_get (`self.MaxTime`))
    (set `self.CurrentTime` 0.0)
    (`KismetSystemLibrary.K2_ClearAndInvalidateTimerHandle` (`self.PlayedTimer`))
    (`GameplayStatics.SetGlobalTimeDilation` 1.0)))

(fn `TimerStart`
  (params (Duration :type "Float (double-precision)"))
  (set `self.MaxTime` Duration)
  (bind _returnvalue (`KismetSystemLibrary.K2_SetTimer` null "PlayingTimer" 0.02 true))
  (set `self.PlayedTimer` _returnvalue))

(fn `UserConstructionScript`)