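; Anim notify state that triggers an enemy's sword ground shockwave during an animation, for owners derived from BP_EnemyBase.
; On begin, it spawns NS_GroundShockwave at a fixed ground height, pulled back from the sword tip toward the enemy.
; It passes that location, raised vertically, to the sword and calls its ChargingSwordTrace.
; On end, it clears the sword's charging timer.
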(fn `Received_NotifyBegin`
  (params (MeshComp :type "SkeletalMeshComponent Object Reference") (Animation :type "AnimSequenceBase Object Reference") (TotalDuration :type "Float (single-precision)") (EventReference :type "AnimNotifyEventReference Structure (by ref)"))
  (returns (ReturnValue :type Boolean))
  (bind _returnvalue (`ActorComponent.GetOwner` MeshComp))
  (bind _asbp_enemy_base (cast `/Game/HyunBin/DummyBoss/Blueprints/BP_EnemyBase` _returnvalue))
  (bind _sword (`/Game/HyunBin/DummyBoss/Blueprints/BP_EnemyBase.Sword` _asbp_enemy_base))
  (bind _returnvalue_2 (`SceneComponent.K2_GetComponentLocation` (`/Game/HyunBin/DummyBoss/Model/Character/BP_EnemySword.SwordTop` _sword)))
  (bind (_returnvalue_x _returnvalue_y) (`KismetMathLibrary.BreakVector` (+ _returnvalue_2 (* (`KismetMathLibrary.Normal` (- _returnvalue_2 (`Actor.K2_GetActorLocation` _asbp_enemy_base))) -150.0))))
  (bind _returnvalue_3 (`NiagaraFunctionLibrary.SpawnSystemAtLocation` _returnvalue "/Game/HyunBin/VFX/AttackVFX/NS_GroundShockwave.NS_GroundShockwave" (`KismetMathLibrary.MakeVector` _returnvalue_x _returnvalue_y 10.0) (struct) (3.5 3.5 3.5)))
  (bind (_returnvalue_x_2 _returnvalue_y_2 _returnvalue_z) (`KismetMathLibrary.BreakVector` (`SceneComponent.K2_GetComponentLocation` _returnvalue_3)))
  (set `/Game/HyunBin/DummyBoss/Model/Character/BP_EnemySword.ShockwaveLocation` (`KismetMathLibrary.MakeVector` _returnvalue_x_2 _returnvalue_y_2 (+ _returnvalue_z 150.0)) _sword)
  (`/Game/HyunBin/DummyBoss/Model/Character/BP_EnemySword.ChargingSwordTrace` _sword)
  (return true))

(fn `Received_NotifyEnd`
  (params (MeshComp :type "SkeletalMeshComponent Object Reference") (Animation :type "AnimSequenceBase Object Reference") (EventReference :type "AnimNotifyEventReference Structure (by ref)"))
  (returns (ReturnValue :type Boolean))
  (bind _asbp_enemy_base (cast `/Game/HyunBin/DummyBoss/Blueprints/BP_EnemyBase` (`ActorComponent.GetOwner` MeshComp)))
  (`KismetSystemLibrary.K2_ClearAndInvalidateTimerHandle` _asbp_enemy_base (`/Game/HyunBin/DummyBoss/Model/Character/BP_EnemySword.ChargingTimer` (`/Game/HyunBin/DummyBoss/Blueprints/BP_EnemyBase.Sword` _asbp_enemy_base)))
  (return true))