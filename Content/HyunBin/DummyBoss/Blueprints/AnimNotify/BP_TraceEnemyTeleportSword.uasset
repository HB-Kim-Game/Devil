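; Anim notify state that opens a sword trace window during an enemy animation, named for the teleport sword attack.
; On begin, it casts the mesh owner to BP_EnemyBase, turns on its sword trace and plays the teleport world camera shake at the enemy's location.
; On end, it turns the sword trace off.
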(fn `Received_NotifyBegin`
  (params (MeshComp :type "SkeletalMeshComponent Object Reference") (Animation :type "AnimSequenceBase Object Reference") (TotalDuration :type "Float (single-precision)") (EventReference :type "AnimNotifyEventReference Structure (by ref)"))
  (returns (ReturnValue :type Boolean))
  (bind _asbp_enemy_base (cast `/Game/HyunBin/DummyBoss/Blueprints/BP_EnemyBase` (`ActorComponent.GetOwner` MeshComp)))
  (`/Game/HyunBin/DummyBoss/Blueprints/BP_EnemyBase.SetSwordTrace` _asbp_enemy_base true)
  (`GameplayStatics.PlayWorldCameraShake` _asbp_enemy_base "/Game/HyunBin/DummyBoss/Blueprints/CameraShake/BP_EnemyTeleportShake.BP_EnemyTeleportShake_C" (`Actor.K2_GetActorLocation` _asbp_enemy_base) 0.0 5000.0)
  (return true))

(fn `Received_NotifyEnd`
  (params (MeshComp :type "SkeletalMeshComponent Object Reference") (Animation :type "AnimSequenceBase Object Reference") (EventReference :type "AnimNotifyEventReference Structure (by ref)"))
  (returns (ReturnValue :type Boolean))
  (bind _asbp_enemy_base (cast `/Game/HyunBin/DummyBoss/Blueprints/BP_EnemyBase` (`ActorComponent.GetOwner` MeshComp)))
  (`/Game/HyunBin/DummyBoss/Blueprints/BP_EnemyBase.SetSwordTrace` _asbp_enemy_base false)
  (return true))