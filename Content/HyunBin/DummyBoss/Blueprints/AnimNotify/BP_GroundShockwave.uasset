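; Anim notify that spawns the ground shockwave Niagara effect for a BP_EnemyBase sword attack.
; It takes the sword tip position, pulls it back toward the enemy along the actor-to-tip direction, and spawns the enlarged effect at a fixed world height near zero.
; The effect's location, raised slightly, is written to the sword's ShockwaveLocation.
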(fn `Received_Notify`
  (params (MeshComp :type "SkeletalMeshComponent Object Reference") (Animation :type "AnimSequenceBase Object Reference") (EventReference :type "AnimNotifyEventReference Structure (by ref)"))
  (returns (ReturnValue :type Boolean))
  (bind _asbp_enemy_base (cast `/Game/HyunBin/DummyBoss/Blueprints/BP_EnemyBase` (`ActorComponent.GetOwner` MeshComp)))
  (bind _sword (`/Game/HyunBin/DummyBoss/Blueprints/BP_EnemyBase.Sword` _asbp_enemy_base))
  (bind _returnvalue (`SceneComponent.K2_GetComponentLocation` (`/Game/HyunBin/DummyBoss/Model/Character/BP_EnemySword.SwordTop` _sword)))
  (bind (_returnvalue_x _returnvalue_y) (`KismetMathLibrary.BreakVector` (+ _returnvalue (* (`KismetMathLibrary.Normal` (- _returnvalue (`Actor.K2_GetActorLocation` _asbp_enemy_base))) -150.0))))
  (bind _returnvalue_2 (`NiagaraFunctionLibrary.SpawnSystemAtLocation` "/Game/HyunBin/VFX/AttackVFX/NS_GroundShockwave.NS_GroundShockwave" (`KismetMathLibrary.MakeVector` _returnvalue_x _returnvalue_y 10.0) (struct) (3.5 3.5 3.5)))
  (bind (_returnvalue_x_2 _returnvalue_y_2 _returnvalue_z) (`KismetMathLibrary.BreakVector` (`SceneComponent.K2_GetComponentLocation` _returnvalue_2)))
  (set `/Game/HyunBin/DummyBoss/Model/Character/BP_EnemySword.ShockwaveLocation` (`KismetMathLibrary.MakeVector` _returnvalue_x_2 _returnvalue_y_2 (+ _returnvalue_z 25.0)) _sword)
  (return true))