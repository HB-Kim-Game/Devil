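; Enemy projectile that flies in a straight line and deals point damage with an enemy-ball damage type.
; SetAttackTarget aims it once at the target's current location, and Tick moves it forward with a swept move, without homing.
; Overlap damages only Characters whose capsule uses a custom collision channel, building the hit result by hand.
; That damage or any blocking hit spawns a Niagara burst and destroys it; a Niagara trail follows it in flight.
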(event `self.ReceiveBeginPlay`
  (bind _returnvalue (`NiagaraFunctionLibrary.SpawnSystemAttached` "/Game/HyunBin/VFX/Basic_VFX/Custom/Custom_Trail2.Custom_Trail2" (`self.Sphere`) "None" (0.0 0.0 0.0) (struct) "KeepRelativeOffset" true))
  (`SceneComponent.K2_SetRelativeLocation` _returnvalue (0.0 0.0 -90.0) true false))

(event `self.ReceiveActorBeginOverlap`
  (params (OtherActor :type "Actor Object Reference"))
  (bind _ascharacter (cast `Character` OtherActor))
  (if (`|EnumEquality` (`PrimitiveComponent.GetCollisionObjectType` (`Character.CapsuleComponent` _ascharacter)) "ECC_GameTraceChannel2")
    (`KismetSystemLibrary.PrintString` "Damage")
    (bind _returnvalue (`self.K2_GetActorLocation` _ascharacter))
    (set `self.Hit Info` (`GameplayStatics.MakeHitResult` true true 0.0 0.0 _returnvalue _returnvalue _returnvalue _returnvalue null _ascharacter (`Character.Mesh` _ascharacter) "None" "None" 0 0 0 _returnvalue _returnvalue))
    (`GameplayStatics.ApplyPointDamage` _ascharacter 10.0 (`KismetMathLibrary.Normal` (- _returnvalue (`self.K2_GetActorLocation` self))) (`self.Hit Info`) null null "/Game/MinSoo/Blueprints/BP_DT_EnemyBall.BP_DT_EnemyBall_C")
    (`/Engine/EditorBlueprintResources/StandardMacros.IsValid` self
      (:`Is Valid`
        (`self.SpawnDestroyEffect`)))))

(event `self.ReceiveTick`
  (params (DeltaSeconds :type "Float (single-precision)"))
  (`/Engine/EditorBlueprintResources/StandardMacros.IsValid` self
    (:`Is Valid`
      (`self.K2_SetActorLocation` (+ (`self.K2_GetActorLocation`) (* (`self.Speed`) DeltaSeconds (`self.GetActorForwardVector`))) true))))

(event `self.ReceiveHit`
  (params (MyComp :type "PrimitiveComponent Object Reference") (Other :type "Actor Object Reference") (OtherComp :type "PrimitiveComponent Object Reference") (bSelfMoved :type Boolean) (HitLocation :type "Vector Structure") (HitNormal :type "Vector Structure") (NormalImpulse :type "Vector Structure") (Hit :type "HitResult Structure (by ref)"))
  (`/Engine/EditorBlueprintResources/StandardMacros.IsValid` self
    (:`Is Valid`
      (`self.SpawnDestroyEffect`))))

(fn `SetAttackTarget`
  (params (Target :type "Actor Object Reference"))
  (bind _output_get (set `self.AttackTarget` Target))
  (bind _output_get_2 (set `self.TargetLocation` (`self.K2_GetActorLocation` _output_get)))
  (`self.K2_SetActorRotation` (`KismetMathLibrary.MakeRotFromXZ` (`KismetMathLibrary.Normal` (- _output_get_2 (`self.K2_GetActorLocation`))) (`self.GetActorUpVector`))))

(fn `SpawnDestroyEffect`
  (bind _returnvalue (`NiagaraFunctionLibrary.SpawnSystemAtLocation` "/Game/HyunBin/VFX/Basic_VFX/Custom/CustomEffect_2.CustomEffect_2" (`self.K2_GetActorLocation`) (struct) (0.5 0.5 0.5)))
  (`NiagaraComponent.SetCustomTimeDilation` _returnvalue 1.5)
  (`self.K2_DestroyActor`))

(fn `UserConstructionScript`)