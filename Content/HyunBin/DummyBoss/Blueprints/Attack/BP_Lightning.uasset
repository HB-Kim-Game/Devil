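; BP_Lightning is a dummy-boss attack actor that fires one delayed lightning strike at its own location.
; After a timer, it plays audio and an overhead Niagara bolt, then sphere-traces downward and applies point damage to hits on a custom collision object type.
; Player death before the strike cancels the timer and destroys the actor; otherwise it destroys itself when the effect finishes.
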(event `self.ReceiveBeginPlay`
  (bind _returnvalue (`KismetSystemLibrary.K2_SetTimerDelegate` (delegate `SpawnLightning`) 0.75))
  (set `self.LightningHandle` _returnvalue)
  (bind _asbp_my_character (cast `/Game/MinSoo/Blueprints/BP_MyCharacter` (`GameplayStatics.GetPlayerPawn` 0)))
  (set `self.AttackTarget` _asbp_my_character)
  (add `/Game/MinSoo/Blueprints/BP_MyCharacter.PlayerDead` _asbp_my_character (delegate `StopTimer`)))

(event `StopTimer`
  (if (`KismetSystemLibrary.K2_IsValidTimerHandle` (`self.LightningHandle`))
    (`KismetSystemLibrary.K2_ClearAndInvalidateTimerHandle` (`self.LightningHandle`))
    (`self.K2_DestroyActor`)))

(event `SpawnLightning`
  (bind _returnvalue (`self.K2_GetActorLocation`))
  (bind _returnvalue_2 (+ _returnvalue (0.0 0.0 600.0)))
  (`ActorComponent.Activate` (`self.Audio`) true)
  (bind _returnvalue_3 (`NiagaraFunctionLibrary.SpawnSystemAtLocation` "/Game/HyunBin/VFX/AttackVFX/NS_Electricity_R.NS_Electricity_R" _returnvalue_2 (struct) (1.0 1.0 1.0) false))
  (add `NiagaraComponent.OnSystemFinished` _returnvalue_3 (delegate `DestroyEvent`))
  (`KismetSystemLibrary.Delay` 0.25)
  (bind (_outhit _returnvalue_4) (`KismetSystemLibrary.SphereTraceSingle` _returnvalue_2 _returnvalue 25.0 "TraceTypeQuery1"))
  (if _returnvalue_4
    (bind (_bblockinghit _binitialoverlap _time _distance _location _impactpoint _normal _impactnormal _physmat _hitactor _hitcomponent) (`GameplayStatics.BreakHitResult` _outhit))
    (if (`|EnumEquality` (`PrimitiveComponent.GetCollisionObjectType` _hitcomponent) "ECC_GameTraceChannel2")
      (`GameplayStatics.ApplyPointDamage` _hitactor 15.0 (`KismetMathLibrary.Normal` (- (`self.K2_GetActorLocation` (`self.AttackTarget`)) _location)) _outhit null null "/Game/MinSoo/Blueprints/BP_DT_EnemyBall.BP_DT_EnemyBall_C"))))

(event `DestroyEvent`
  (params (PSystem :type "NiagaraComponent Object Reference"))
  (`ActorComponent.K2_DestroyComponent` PSystem)
  (remove `/Game/MinSoo/Blueprints/BP_MyCharacter.PlayerDead` (`self.AttackTarget`) (delegate `StopTimer`))
  (`self.K2_DestroyActor`))

(fn `UserConstructionScript`)