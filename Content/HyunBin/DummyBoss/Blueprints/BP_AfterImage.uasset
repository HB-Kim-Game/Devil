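; BP_AfterImage is a short-lived afterimage actor that leaves a frozen copy of an enemy's pose.
; SetCharacter stores the target, and Activate casts it to BP_EnemyBase, copies its skeletal mesh and current pose onto a PoseableMesh, and applies the M_AfterImage material.
; A random material parameter varies each image, while a Timeline drives the Alpha parameter before the actor destroys itself after a brief delay.
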(event `Activate`
  (bind _poseablemesh (`self.PoseableMesh`))
  (bind _poseablemesh_2 (`self.PoseableMesh`))
  (bind _asbp_enemy_base (cast `/Game/HyunBin/DummyBoss/Blueprints/BP_EnemyBase` (`self.Character`)))
  (bind _mesh (`Character.Mesh` _asbp_enemy_base))
  (`SkinnedMeshComponent.SetSkinnedAssetAndUpdate` _poseablemesh (`SkeletalMeshComponent.SkeletalMeshAsset` _mesh) true)
  (`PrimitiveComponent.SetMaterial` _poseablemesh 0 "/Game/HyunBin/DummyBoss/Material/M_AfterImage.M_AfterImage")
  (`PrimitiveComponent.SetMaterial` _poseablemesh 1 "/Game/HyunBin/DummyBoss/Material/M_AfterImage.M_AfterImage")
  (`MeshComponent.SetScalarParameterValueOnMaterials` _poseablemesh_2 "Random" (`KismetMathLibrary.RandomFloat`))
  (`PoseableMeshComponent.CopyPoseFromSkeletalComponent` _poseablemesh_2 _mesh)
  (bind (_direction _newtrack_0) (`Timeline|Timeline` :!via `PlayFromStart`)
    (:`Update`
      (`MeshComponent.SetScalarParameterValueOnMaterials` (`self.PoseableMesh`) "Alpha" _newtrack_0))
    (:`Finished`
      (`KismetSystemLibrary.Delay` 0.2)
      (`self.K2_DestroyActor`))))

(fn `SetCharacter`
  (params (TargetCharacter :type "Pawn Object Reference"))
  (set `self.Character` TargetCharacter))

(fn `UserConstructionScript`)