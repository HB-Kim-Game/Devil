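; BP_Test is a test Character in the DummyBoss folder that performs a single charge toward the player.
; Tick passes through a DoOnce into a three-second delay, then raises walk speed, turns the actor to face the player pawn and calls LaunchCharacter.
; The launch follows the normalized horizontal direction to the player, scaled by mesh mass and a large constant.
; A SimpleMoveToLocation node is left unconnected.
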(event `self.ReceiveTick`
  (params (DeltaSeconds :type "Float (single-precision)"))
  (bind _returnvalue (`KismetMathLibrary.Vector_Normal2D` (- (`self.K2_GetActorLocation` (`GameplayStatics.GetPlayerPawn` 0)) (`self.K2_GetActorLocation`))))
  (`/Engine/EditorBlueprintResources/StandardMacros.DoOnce` false
    (:`Completed`
      (`KismetSystemLibrary.Delay` 3.0)
      (set `CharacterMovementComponent.MaxWalkSpeed` 2000.0 (`self.CharacterMovement`))
      (`self.K2_SetActorRotation` (`KismetMathLibrary.MakeRotFromXZ` _returnvalue (`self.GetActorUpVector`)))
      (`self.LaunchCharacter` (* _returnvalue (`PrimitiveComponent.GetMass` (`self.Mesh`)) 2000.0)))))

(event `self.ReceiveBeginPlay`)

(fn `UserConstructionScript`)