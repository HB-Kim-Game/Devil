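; BP_TestTimer is a test timer actor that unpauses the game after a given duration.
; TimerStart stores the duration and raises IsStart, and Tick, set to run while paused, accumulates delta seconds until that limit.
; It then calls SetGamePaused(false), zeroes the counter and assigns that call's return value to IsStart, rather than clearing the flag explicitly.
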(event `self.ReceiveBeginPlay`
  (`self.SetTickableWhenPaused` true))

(event `self.ReceiveTick`
  (params (DeltaSeconds :type "Float (single-precision)"))
  (if (`self.IsStart`)
    (bind _output_get (set `self.CurrentTime` (+ (`self.CurrentTime`) DeltaSeconds)))
    (if (>= _output_get (`self.MaxTime`))
      (bind _returnvalue (`GameplayStatics.SetGamePaused` false))
      (set `self.IsStart` _returnvalue)
      (set `self.CurrentTime` 0.0))))

(fn `TimerStart`
  (params (Duration :type "Float (double-precision)"))
  (set `self.MaxTime` Duration)
  (set `self.IsStart` true))

(fn `UserConstructionScript`)