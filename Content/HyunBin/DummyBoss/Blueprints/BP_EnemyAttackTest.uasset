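; BP_EnemyAttackTest is a test enemy Blueprint in the DummyBoss folder that fires a projectile at the player.
; Attack spawns a BP_EnemyProjectile at the skeletal mesh's LeftHand socket, ignoring collisions, then sweeps it slightly along its forward vector.
; It passes player character 0 to the projectile as its attack target.
; The event graph and construction script are empty, so nothing in this Blueprint calls Attack.
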(fn `Attack`
  (bind _returnvalue (`|SpawnActorFromClass` "/Game/HyunBin/DummyBoss/Blueprints/BP_EnemyProjectile.BP_EnemyProjectile_C" (`SceneComponent.GetSocketTransform` (`self.SkeletalMesh`) "LeftHand" "RTS_World") "AlwaysSpawn" "MultiplyWithRoot" null null))
  (`self.K2_SetActorLocation` _returnvalue (+ (* (`self.GetActorForwardVector` _returnvalue) 20.0) (`self.K2_GetActorLocation` _returnvalue)) true false)
  (`/Game/HyunBin/DummyBoss/Blueprints/BP_EnemyProjectile.SetAttackTarget` _returnvalue (`GameplayStatics.GetPlayerCharacter` 0)))

(fn `UserConstructionScript`)