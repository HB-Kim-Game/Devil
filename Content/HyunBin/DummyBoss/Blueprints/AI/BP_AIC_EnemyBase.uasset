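; Base enemy AI controller that runs BT_EnemyBase on possess and drives its blackboard state and attack radii.
; Perception updates send sight, hearing and damage to handlers that switch Passive or Investigating enemies to Attacking or Investigating.
; Helper functions turn accumulated damage into Armor, Default or Stun hit states for Frozen reactions, and manage randomized strafing and ball-attack counts.
; Player death stops the brain logic, and continue restarts it after a delay.
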(event `self.ReceivePossess`
  (params (PossessedPawn :type "Pawn Object Reference"))
  (bind _blackboard (`self.Blackboard`))
  ; Behavior Tree를 작동시키고 블랙보드에 값 설정
  (`self.RunBehaviorTree` "/Game/HyunBin/DummyBoss/Blueprints/AI/BT_EnemyBase.BT_EnemyBase")
  (`self.SetStateAsPassive`)
  (bind (_attackradius _defendradius) (message `/Game/HyunBin/DummyBoss/Blueprints/AI/BPI_EnemyAI.GetIdealRange` PossessedPawn))
  (`BlackboardComponent.SetValueAsFloat` _blackboard (`self.AttackRadiusKeyName`) _attackradius)
  (`BlackboardComponent.SetValueAsFloat` _blackboard (`self.DefendRadiusKeyName`) _defendradius))

(event `self.AIPerception.OnPerceptionUpdated`
  (params (UpdatedActors :type "Array of Actor Object Reference (by ref)"))
  ; AI가 감지를 했을때,감지한 Actors 배열 반환
  (for _array_element UpdatedActors
    (`|ExecutionSequence`
      (:`then_0`
        ; 시각 감지
        (bind _sensed (`self.CanSenseActor` _array_element "NewEnumerator1"))
        (if _sensed
          (`self.HandleSight` _array_element)))
      (:`then_1`
        ; 청각 감지
        (bind (_sensed_2 _stimulus) (`self.CanSenseActor` _array_element "NewEnumerator2"))
        (if _sensed_2
          (`self.HandleHearing` (`.StimulusLocation` (break `AIStimulus` _stimulus)))))
      (:`then_2`
        ; 데미지 감지
        (bind _sensed_3 (`self.CanSenseActor` _array_element "NewEnumerator3"))
        (if _sensed_3
          (`self.HandleDamage` _array_element))))))

(event `self.ReceiveBeginPlay`
  (bind _asbp_my_character (cast `/Game/MinSoo/Blueprints/BP_MyCharacter` (`GameplayStatics.GetPlayerPawn` 0)))
  (add `/Game/MinSoo/Blueprints/BP_MyCharacter.PlayerDead` _asbp_my_character (delegate `OnPlayerDead`))
  (add `/Game/MinSoo/Blueprints/BP_MyCharacter.PlayerContinue` _asbp_my_character (delegate `OnPlayerContinue`)))

(event `OnPlayerDead`
  (`BrainComponent.StopLogic` (`self.BrainComponent`) ""))

(event `OnPlayerContinue`
  (`KismetSystemLibrary.Delay` 1.0)
  (`BrainComponent.RestartLogic` (`self.BrainComponent`)))

(fn `AddDamage`
  (params (Damage :type "Float (double-precision)"))
  (switch `/Game/HyunBin/DummyBoss/Blueprints/AI/Enum/E_HitState` (cast `/Game/HyunBin/DummyBoss/Blueprints/AI/Enum/E_HitState` (`BlackboardComponent.GetValueAsEnum` (`self.Blackboard`) (`self.HitStateKeyName`)))
    (:`NewEnumerator0`
      _)
    (:`NewEnumerator1`
      _))
  (set `self.HitStateDamage` (+ Damage (`self.HitStateDamage`))))

(fn `CanSenseActor`
  (params (Actor :type "Actor Object Reference") (Sense :type "/Game/HyunBin/DummyBoss/Blueprints/AI/Enum/E_AISense Enum" :default "NewEnumerator0"))
  (returns (Sensed :type Boolean) (Stimulus :type "AIStimulus Structure"))
  ; AI 감각을 확인
  (bind _info (`AIPerceptionComponent.GetActorsPerception` (`self.AIPerception`) Actor))
  (for _array_element (`.LastSensedStimuli` (break `ActorPerceptionBlueprintInfo` _info))
    ; 느낀 감각과 확인하려는 감각이 같은지 확인 (시각,청각,데미지중 하나)
    (bind _returnvalue (`AIPerceptionSystem.GetSenseClassForStimulus` _array_element))
    (if (== _returnvalue (select `/Game/HyunBin/DummyBoss/Blueprints/AI/Enum/E_AISense` Sense :`NewEnumerator1` "/Script/AIModule.AISense_Sight" :`NewEnumerator2` "/Script/AIModule.AISense_Hearing" :`NewEnumerator3` "/Script/AIModule.AISense_Damage" :!type "Object Class Reference"))
      (return (`.bSuccessfullySensed` (break `AIStimulus` _array_element)) _array_element))))

(fn `CheckBallCount`
  (bind _result (`/Engine/EditorBlueprintResources/StandardMacros.IncrementInt` (`self.BallAttackCount`))
    (:`  `
      (bind _output_get (set `self.BallAttackCount` _result))
      (if (>= _output_get (`self.MaxBallAttackCount`))
        (`self.ClearStrafeState`)
        (`self.InvertDefaultAttack`)
        (set `self.BallAttackCount` 0)))))

(fn `ClearBallAttack`
  (set `self.BallAttackCount` 0))

(fn `ClearDamage`
  (set `self.HitStateDamage` 0.0)
  (`KismetSystemLibrary.PrintString` "Hello" true true (struct :`G` 0.66 :`B` 1.0 :`A` 1.0) (`self.HitStateDamage`)))

(fn `ClearStrafeState`
  (`BlackboardComponent.SetValueAsEnum` (`self.Blackboard`) (`self.StrafeStateKeyName`) (enumliteral `/Game/HyunBin/DummyBoss/Blueprints/AI/Enum/E_StrafeState` "NewEnumerator0")))

(fn `GetCurrentState`
  (returns (State :type "/Game/HyunBin/DummyBoss/Blueprints/AI/Enum/E_EnemyState Enum"))
  (return (cast `/Game/HyunBin/DummyBoss/Blueprints/AI/Enum/E_EnemyState` (`BlackboardComponent.GetValueAsEnum` (`self.Blackboard`) (`self.StateKeyName`)))))

(fn `HandleDamage`
  (params (Actor :type "Actor Object Reference"))
  (bind _state (`self.GetCurrentState`))
  (switch `/Game/HyunBin/DummyBoss/Blueprints/AI/Enum/E_EnemyState` _state
    (:`NewEnumerator0`
      _)
    (:`NewEnumerator3`
      _))
  (`self.SetStateAsAttacking` Actor))

(fn `HandleHearing`
  (params (Location :type "Vector Structure"))
  (bind _state (`self.GetCurrentState`))
  (switch `/Game/HyunBin/DummyBoss/Blueprints/AI/Enum/E_EnemyState` _state
    (:`NewEnumerator0`
      _)
    (:`NewEnumerator3`
      _))
  (`self.SetStateAsInvestigating` Location))

(fn `HandleSight`
  (params (Actor :type "Actor Object Reference"))
  (bind _state (`self.GetCurrentState`))
  (switch `/Game/HyunBin/DummyBoss/Blueprints/AI/Enum/E_EnemyState` _state
    (:`NewEnumerator0`
      _)
    (:`NewEnumerator3`
      _))
  (if (== Actor (`GameplayStatics.GetPlayerCharacter` 0))
    (`self.SetStateAsAttacking` Actor)))

(fn `InvertDefaultAttack`
  (bind _blackboard (`self.Blackboard`))
  (bind _defaultattackkeyname (`self.DefaultAttackKeyName`))
  (`BlackboardComponent.SetValueAsBool` _blackboard _defaultattackkeyname (not (`BlackboardComponent.GetValueAsBool` _blackboard _defaultattackkeyname))))

(fn `SetHitState`
  (bind _hitstatekeyname (`self.HitStateKeyName`))
  (bind _blackboard (`self.Blackboard`))
  (if (>= (`self.HitStateDamage`) (`self.ArmorClearDamage`))
    (if (>= (`self.HitStateDamage`) (`self.StunDamage`))
      (`BlackboardComponent.SetValueAsEnum` _blackboard _hitstatekeyname (enumliteral `/Game/HyunBin/DummyBoss/Blueprints/AI/Enum/E_HitState` "NewEnumerator2"))
      (else
        (`BlackboardComponent.SetValueAsEnum` _blackboard _hitstatekeyname (enumliteral `/Game/HyunBin/DummyBoss/Blueprints/AI/Enum/E_HitState` "NewEnumerator1"))))
    (else
      (`BlackboardComponent.SetValueAsEnum` _blackboard _hitstatekeyname (enumliteral `/Game/HyunBin/DummyBoss/Blueprints/AI/Enum/E_HitState` "NewEnumerator0")))))

(fn `SetMaxBallCount`
  (if (<= (`self.BallAttackCount`) 0)
    (set `self.MaxBallAttackCount` (`KismetMathLibrary.RandomIntegerInRange` 1 3))))

(fn `SetStateAsAttacking`
  (params (AttackTarget :type "Actor Object Reference"))
  (`BlackboardComponent.SetValueAsObject` (`self.Blackboard`) (`self.AttackTargetName`) AttackTarget)
  (`BlackboardComponent.SetValueAsEnum` (`self.Blackboard`) (`self.StateKeyName`) (enumliteral `/Game/HyunBin/DummyBoss/Blueprints/AI/Enum/E_EnemyState` "NewEnumerator1"))
  (set `self.Attack Target` AttackTarget))

(fn `SetStateAsDead`
  (`BlackboardComponent.SetValueAsEnum` (`self.Blackboard`) (`self.StateKeyName`) (enumliteral `/Game/HyunBin/DummyBoss/Blueprints/AI/Enum/E_EnemyState` "NewEnumerator4")))

(fn `SetStateAsFrozen`
  (bind _blackboard (`self.Blackboard`))
  (bind _statekeyname (`self.StateKeyName`))
  (`self.SetHitState`)
  (switch `/Game/HyunBin/DummyBoss/Blueprints/AI/Enum/E_HitState` (cast `/Game/HyunBin/DummyBoss/Blueprints/AI/Enum/E_HitState` (`BlackboardComponent.GetValueAsEnum` (`self.Blackboard`) (`self.HitStateKeyName`)))
    (:`NewEnumerator1`
      (`BlackboardComponent.SetValueAsEnum` _blackboard _statekeyname (enumliteral `/Game/HyunBin/DummyBoss/Blueprints/AI/Enum/E_EnemyState` "NewEnumerator0") :!label _label)
      (`BlackboardComponent.SetValueAsEnum` _blackboard _statekeyname (enumliteral `/Game/HyunBin/DummyBoss/Blueprints/AI/Enum/E_EnemyState` "NewEnumerator2")))
    (:`NewEnumerator2`
      (if (`|EnumInequality` (cast `/Game/HyunBin/DummyBoss/Blueprints/AI/Enum/E_EnemyState` (`BlackboardComponent.GetValueAsEnum` (`self.Blackboard`) (`self.StateKeyName`))) "NewEnumerator2")
        (goto _label)))))

(fn `SetStateAsInvestigating`
  (params (Location :type "Vector Structure"))
  (`BlackboardComponent.SetValueAsEnum` (`self.Blackboard`) (`self.StateKeyName`) (enumliteral `/Game/HyunBin/DummyBoss/Blueprints/AI/Enum/E_EnemyState` "NewEnumerator3"))
  (`BlackboardComponent.SetValueAsVector` (`self.Blackboard`) (`self.InterestPointKeyName`) Location))

(fn `SetStateAsPassive`
  (`BlackboardComponent.SetValueAsEnum` (`self.Blackboard`) (`self.StateKeyName`) (enumliteral `/Game/HyunBin/DummyBoss/Blueprints/AI/Enum/E_EnemyState` "NewEnumerator0")))

(fn `SetStrafeState`
  (bind _blackboard (`self.Blackboard`))
  (bind _strafestatekeyname (`self.StrafeStateKeyName`))
  (if (< (`KismetMathLibrary.RandomIntegerInRange` 0 9) 4)
    (`BlackboardComponent.SetValueAsEnum` _blackboard _strafestatekeyname (enumliteral `/Game/HyunBin/DummyBoss/Blueprints/AI/Enum/E_StrafeState` "NewEnumerator2"))
    (else
      (`BlackboardComponent.SetValueAsEnum` _blackboard _strafestatekeyname (enumliteral `/Game/HyunBin/DummyBoss/Blueprints/AI/Enum/E_StrafeState` "NewEnumerator1")))))

(fn `UserConstructionScript`)